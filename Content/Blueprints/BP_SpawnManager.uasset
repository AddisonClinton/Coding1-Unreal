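; BP_SpawnManager runs endless enemy waves, starting the first shortly after BeginPlay.
; SpawnEnemies loops over every BP_SpawnPoint and spawns a BP_Enemy at its transform with a weighted random chance, so some points stay empty.
; NewWaveCheck, intended to be called by dying enemies, counts remaining BP_Enemy actors and respawns after a delay when at most one remains.
; Debug PrintString messages trace each step.
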(event Custom|Spawn%20Enemies
  (bind _outactors (Actor|GetAllActorsOfClass "/Game/Blueprints/BP_SpawnPoint.BP_SpawnPoint_C")) ; get an array of all spawnpoints in the level
  (for _array_element _outactors
    (Development|PrintString (Utilities|GetDisplayName _array_element) true true "(R=1.000000,G=0.970354,B=0.000000,A=1.000000)" 1e+01)
    (if (Math|Random|RandomBoolwithWeight 0.8) ; chance to not spawn an enemy
      (Game|SpawnActorfromClass "/Game/Blueprints/BP_Enemy.BP_Enemy_C" (Transformation|GetWorldTransform (Variables|/Game/Blueprints/BP_SpawnPoint.BP_SpawnPoint_C|GetDefaultSceneRoot _array_element)) "Undefined" "MultiplyWithRoot" 0 0)))
  (Development|PrintString "finished with the For Each loop for spawning enemies"))

(event Custom|NewWaveCheck
  (Development|PrintString "Was I the last one???")
  (bind _outactors (Actor|GetAllActorsOfClass "/Game/Blueprints/BP_Enemy.BP_Enemy_C"))
  (Development|PrintString (Utilities|String|Append "There are" (Utilities|String|ToString(Integer) (Utilities|Array|Length _outactors)) " enemies left"))
  (if (> (Utilities|Array|Length _outactors) 1) ; are there more than 0 enemies?
    (Development|PrintString "you are not the last one")
    (else
      (Utilities|FlowControl|Delay 3.0)
      (CallFunction|SpawnEnemies))))

(event EventBeginPlay
  (Development|PrintString "Spawn Manager exists") ; tell the player that we exist
  (Utilities|FlowControl|Delay 1.0)
  (CallFunction|SpawnEnemies))

(fn ConstructionScript)