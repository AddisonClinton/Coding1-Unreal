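; A falling platform that drops after the Custom3rdperson character touches its trigger box, then returns to its starting transform.
; Custom events chain activated, falling and resetting stages through delays, each swapping the platform material to show its state.
; The fall uses physics simulation, then a timeline lerps the platform from its fallen transform back to the one saved at BeginPlay.
; An IsReady flag blocks retriggering until the return finishes.
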(event OnComponentBeginOverlap(Box)
  (params (OverlappedComponent :type Primitive%20Component%20Object%20Reference) (OtherActor :type Actor%20Object%20Reference) (OtherComp :type Primitive%20Component%20Object%20Reference) (OtherBodyIndex :type Integer) (bFromSweep :type Boolean) (SweepResult :type Hit%20Result%20Structure%20%28by%20ref%29))
  ;[0.15 0.15 0.15 0.5] Comment
  (Development|PrintString "the box has been touched")
  (if (Variables|Default|GetisReady)
    (Utilities|Casting|CastToCustom3rdperson OtherActor)
    (CallFunction|Avtivated)))

(event Custom|Avtivated
  ;[0.15 0.15 0.15 0.5] activated
  (Development|PrintString "activated")
  (Rendering|Material|SetMaterial (Variables|Default|GetPlatform) 0 "/Game/Materials/PlatformMats/MI_Platform_Activated.MI_Platform_Activated")
  (Variables|Default|SetisReady false)
  (Utilities|FlowControl|Delay (Variables|Default|GetFallDelayDuration))
  (CallFunction|Falling))

(event Custom|Falling
  ;[0.15 0.15 0.15 0.5] falling
  (Development|PrintString "falling")
  (Rendering|Material|SetMaterial (Variables|Default|GetPlatform) 0 "/Game/Materials/PlatformMats/MI_Platform_Falling.MI_Platform_Falling")
  (Physics|SetSimulatePhysics (Variables|Default|GetPlatform) true)
  (Utilities|FlowControl|Delay 3.0)
  (CallFunction|Resetting))

(event Custom|Resetting
  ;[0.15 0.15 0.15 0.5] resetting
  (Development|PrintString "resetting")
  (Rendering|Material|SetMaterial (Variables|Default|GetPlatform) 0 "/Game/Materials/PlatformMats/MI_Platform_Resetting.MI_Platform_Resetting")
  (Variables|Default|Setfallentransform (Transformation|GetWorldTransform (Variables|Default|GetPlatform)))
  (Physics|SetSimulatePhysics (Variables|Default|GetPlatform) false)
  (bind _newtrack_0 (Timeline|returntostart PlayFromStart)
    (:Update
      (Transformation|SetWorldLocationAndRotation (Variables|Default|GetPlatform) (.location (Math|Transform|Lerp(Transform) (Variables|Default|Getfallentransform) (Variables|Default|Getoriginaltransform) _newtrack_0)) (.rotation (Math|Transform|Lerp(Transform) (Variables|Default|Getfallentransform) (Variables|Default|Getoriginaltransform) _newtrack_0)) false false))
    (:Finished
      (Rendering|Material|SetMaterial (Variables|Default|GetPlatform) 0 "/Game/Materials/PlatformMats/MI_Platform_Ready.MI_Platform_Ready")
      (Variables|Default|SetisReady true))))

(event EventBeginPlay
  ;[0.15 0.15 0.15 0.5] Comment
  (Variables|Default|Setoriginaltransform (Transformation|GetWorldTransform (Variables|Default|GetPlatform)))
  (Rendering|Material|SetMaterial (Variables|Default|GetPlatform) 0 "/Game/Materials/PlatformMats/MI_Platform_Ready.MI_Platform_Ready"))

(fn ConstructionScript)